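; Motion controller actor that follows the player pawn every tick and registers shuriken hits on left and right boxes.
; Either box hit plays a sound, using NormalImpulse as its location, and side-specific force feedback.
; Both then share a path that marks the SyurikenActor dead and calls UpdateSyurikenState on BP_PlayerPawn.
; That path reads OtherActor only from the right box's event, even for left hits.
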(event `self.ReceiveTick`
  (params (DeltaSeconds :type "Float (single-precision)"))
  (`self.K2_SetActorLocation` (`self.K2_GetActorLocation` (`GameplayStatics.GetPlayerPawn` 0))))

(event `self.BoxRight.OnComponentHit`
  (params (HitComponent :type "PrimitiveComponent Object Reference") (OtherActor :type "Actor Object Reference") (OtherComp :type "PrimitiveComponent Object Reference") (NormalImpulse :type "Vector Structure") (Hit :type "HitResult Structure (by ref)"))
  (`GameplayStatics.PlaySoundAtLocation` "/Game/Game/Audio/ShirikenHit.ShirikenHit" NormalImpulse)
  (`PlayerController.ClientPlayForceFeedback` (`GameplayStatics.GetPlayerController` 0) "/Game/Game/Blueprints/Player/FFE_DartRight.FFE_DartRight" false "None")
  (bind _assyuriken_actor (cast `/Game/Game/Blueprints/SyurikenActor` OtherActor :!label _label))
  (set `/Game/Game/Blueprints/SyurikenActor.IsDead` true _assyuriken_actor)
  (bind _asbp_player_pawn (cast `/Game/Game/Blueprints/BP_PlayerPawn` (`GameplayStatics.GetPlayerPawn` 0)))
  (`/Game/Game/Blueprints/BP_PlayerPawn.UpdateSyurikenState` _asbp_player_pawn))

(event `self.BoxLeft.OnComponentHit`
  (params (HitComponent :type "PrimitiveComponent Object Reference") (OtherActor :type "Actor Object Reference") (OtherComp :type "PrimitiveComponent Object Reference") (NormalImpulse :type "Vector Structure") (Hit :type "HitResult Structure (by ref)"))
  (`GameplayStatics.PlaySoundAtLocation` "/Game/Game/Audio/ShirikenHit.ShirikenHit" NormalImpulse)
  (`PlayerController.ClientPlayForceFeedback` (`GameplayStatics.GetPlayerController` 0) "/Game/Game/Blueprints/Player/FFE_DartLeft.FFE_DartLeft" false "None")
  (goto _label))

(fn `UserConstructionScript`)