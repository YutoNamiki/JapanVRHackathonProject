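; SpawnCharacterActor is a timed spawner that places characters at its own transform.
; Tick accumulates elapsed time and scans the SpawnInfo list for entries whose appearance time has arrived.
; Each due entry spawns its character type, adjusting for collisions but always spawning, and gives it a default controller.
; Spawned entries are removed from SpawnInfo inside the same loop that iterates over it.
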(event `self.ReceiveTick`
  (params (DeltaSeconds :type "Float (single-precision)"))
  (set `self.Time` (+ DeltaSeconds (`self.Time`)))
  (for _array_element (`self.SpawnInfo`)
    (bind (_charactertype _appearancetime) (break `/Game/Game/Blueprints/SpawnCharacterInfo` _array_element))
    (if (<= _appearancetime (`self.Time`))
      (bind _returnvalue (`|SpawnActorFromClass` _charactertype (`self.GetTransform`) "AdjustIfPossibleButAlwaysSpawn" "OverrideRootScale"))
      (`Pawn.SpawnDefaultController` _returnvalue)
      (`KismetArrayLibrary.Array_RemoveItem` (`self.SpawnInfo`) _array_element))))

(fn `UserConstructionScript`)