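; A double sliding door actor that opens when any actor begins overlapping it and closes when an overlap ends.
; Open plays DoorTimeline, whose Left vector track sets the relative locations of MovableDoor1 and MovableDoor2, each added to its own offset.
; MovableDoor1 uses the same track with X negated, so the panels mirror each other.
; Close reverses the same timeline.
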(event `self.ReceiveBeginPlay`)

(event `self.ReceiveActorBeginOverlap`
  (params (OtherActor :type "Actor Object Reference"))
  (`self.Open`))

(event `self.ReceiveActorEndOverlap`
  (params (OtherActor :type "Actor Object Reference"))
  (`self.Close`))

(event `Open`
  (bind (_direction _left) (`Timeline|DoorTimeline` :!label _label)
    (:`Update`
      (`SceneComponent.K2_SetRelativeLocation` (`self.MovableDoor2`) (+ _left (`self.Door2Offset`)) false false)
      (`SceneComponent.K2_SetRelativeLocation` (`self.MovableDoor1`) (+ (* _left (-1.0 1.0 1.0)) (`self.Door1Offset`)) false false))))

(event `Close`
  (goto _label :!via `Reverse`))

(fn `UserConstructionScript`)