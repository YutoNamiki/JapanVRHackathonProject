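; MainGameState holds two running values for the game: elapsed time and a repel count.
; Tick adds the frame delta to Time, which GetTime exposes.
; AddRepelCount increases RepelCount by a given amount, and GetRepelCount returns the total.
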(event `self.ReceiveTick`
  (params (DeltaSeconds :type "Float (single-precision)"))
  (set `self.Time` (+ DeltaSeconds (`self.Time`))))

(fn `AddRepelCount`
  (params (AddCount :type Integer))
  (set `self.RepelCount` (+ AddCount (`self.RepelCount`)))
  (return))

(fn `GetRepelCount`
  (returns (Count :type Integer))
  (return (`self.RepelCount`)))

(fn `GetTime`
  (returns (Time :type "Float (double-precision)"))
  (return (`self.Time`)))

(fn `UserConstructionScript`)