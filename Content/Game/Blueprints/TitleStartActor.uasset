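; TitleStartActor is an actor, apparently the title screen's start trigger, that the player activates by touch or sword strike.
; Its static mesh rotates in local pitch every Tick at RotateSpeed.
; An overlap with a BP_MotionController, or a hit from a component using the sword collision profile, enables physics simulation on the Sphere and sets the IsStart flag.
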(event `self.ReceiveTick`
  (params (DeltaSeconds :type "Float (single-precision)"))
  (`SceneComponent.K2_AddLocalRotation` (`self.StaticMesh`) (`KismetMathLibrary.MakeRotator` 0.0 (* DeltaSeconds (`self.RotateSpeed`))) false false))

(event `self.ReceiveActorBeginOverlap`
  (params (OtherActor :type "Actor Object Reference"))
  (cast `/Game/Game/Blueprints/Player/BP_MotionController` OtherActor)
  (`PrimitiveComponent.SetSimulatePhysics` (`self.Sphere`) true :!label _label)
  (set `self.IsStart` true))

(event `self.ReceiveHit`
  (params (MyComp :type "PrimitiveComponent Object Reference") (Other :type "Actor Object Reference") (OtherComp :type "PrimitiveComponent Object Reference") (bSelfMoved :type Boolean) (HitLocation :type "Vector Structure") (HitNormal :type "Vector Structure") (NormalImpulse :type "Vector Structure") (Hit :type "HitResult Structure (by ref)"))
  (bind _returnvalue (`PrimitiveComponent.GetCollisionProfileName` OtherComp))
  (if (== _returnvalue (`self.SwordProfile`))
    (goto _label)))

(fn `UserConstructionScript`)