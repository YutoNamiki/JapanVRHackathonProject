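; BP_PlayerPawn is the player's VR pawn, which triggers slow motion when a live shuriken is near.
; It spawns a motion controller on BeginPlay and exposes headset-based player location and forward vector.
; Sphere overlap changes rescan for live SyurikenActors and tell MainGameMode to slow or restore global time.
; The pawn copies the game mode's global time changes into its own CustomTimeDilation.
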(event OnComponentBeginOverlap(Sphere)
  (params (OverlappedComponent :type Primitive%20Component%20Object%20Reference) (OtherActor :type Actor%20Object%20Reference) (OtherComp :type Primitive%20Component%20Object%20Reference) (OtherBodyIndex :type Integer) (bFromSweep :type Boolean) (SweepResult :type Hit%20Result%20Structure%20%28by%20ref%29))
  (bind _assyuriken_actor (Utilities|Casting|CastToSyurikenActor OtherActor))
  (if (not (Variables|/Game/Game/Blueprints/SyurikenActor.SyurikenActor_C|GetIsDead _assyuriken_actor))
    (CallFunction|UpdateSyurikenState)))

(event OnComponentEndOverlap(Sphere)
  (params (OverlappedComponent :type Primitive%20Component%20Object%20Reference) (OtherActor :type Actor%20Object%20Reference) (OtherComp :type Primitive%20Component%20Object%20Reference) (OtherBodyIndex :type Integer))
  (Utilities|Casting|CastToSyurikenActor OtherActor)
  (CallFunction|UpdateSyurikenState))

(event Custom|OnChangeGlobalTime_Event_0
  (params (Scale :type Float%20%28single-precision%29))
  (Variables|Default|SetCustomTimeDilation Scale))

(event EventBeginPlay
  (Game|SpawnActorfromClass "/Game/Game/Blueprints/Player/BP_MotionController.BP_MotionController_C" (Math|Transform|MakeTransform "0, 0, 0") "Undefined" 0 0)
  (bind _asmain_game_mode (Utilities|Casting|CastToMainGameMode (Game|GetGameMode)))
  (EventDispatchers|AssignOnChangeGlobalTime _asmain_game_mode (delegate Custom|OnChangeGlobalTime_Event_0)))

(event Collision|EventActorBeginOverlap
  (params (OtherActor :type Actor%20Object%20Reference)))

(event EventTick
  (params (DeltaSeconds :type Float%20%28single-precision%29)))

(fn ConstructionScript)

(fn GetPlayerLocation
  (bind (_devicerotation _deviceposition) (Class|HeadMountedDisplayFunctionLibrary|GetOrientationandPosition))
  (return (Math|Transform|TransformLocation (Transformation|GetActorTransform (Game|GetPlayerCameraManager 0)) (Math|Vector|UnrotateVector _deviceposition _devicerotation))))

(fn UpdateSyurikenState
  (bind _array_element (Utilities|Array|ForEachLoopwithBreak (Collision|GetOverlappingActors (Variables|Default|GetSphere) "/Game/Game/Blueprints/SyurikenActor.SyurikenActor_C" :!class /Script/Engine.PrimitiveComponent) :!label _label)
    (:LoopBody
      (bind _assyuriken_actor (Utilities|Casting|CastToSyurikenActor _array_element))
      (if (not (Variables|/Game/Game/Blueprints/SyurikenActor.SyurikenActor_C|GetIsDead _assyuriken_actor))
        (bind _asmain_game_mode (Utilities|Casting|CastToMainGameMode (Game|GetGameMode)))
        (Default|SetGlobalTime _asmain_game_mode 0.1)
        (LocalVariables|SetbSlow true)
        (goto _label Break)))
    (:Completed
      (if (LocalVariables|GetbSlow)
        _
        (else
          (bind _asmain_game_mode_2 (Utilities|Casting|CastToMainGameMode (Game|GetGameMode)))
          (Default|SetGlobalTime _asmain_game_mode_2 1.0)))
      (return))))

(fn GetPlayerForwardVector
  (return (Math|Vector|GetForwardVector (.DeviceRotation (Class|HeadMountedDisplayFunctionLibrary|GetOrientationandPosition)))))